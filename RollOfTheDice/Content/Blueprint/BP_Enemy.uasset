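; BP_Enemy is an enemy pawn that chases a target actor.
; On BeginPlay it targets the Dice_Blueprint actor, and AI perception updates switch the target to any reported ThirdPersonCharacter.
; Tick reissues AI Move To toward the target's location every frame while the target is valid.
; Any damage prints a debug string, and only a hit of at least CurrentHP destroys the enemy, as CurrentHP is never reduced here.
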(event OnTargetPerceptionUpdated(AIPerception)
  (params (Actor :type Actor%20Object%20Reference) (Stimulus :type AI%20Stimulus%20Structure))
  (bind _asthird_person_character (Utilities|Casting|CastToThirdPersonCharacter Actor))
  (Variables|Default|SettargetActor _asthird_person_character))

(event EventBeginPlay
  (bind _returnvalue (Actor|GetActorOfClass "/Game/Dice/Dice_Blueprint.Dice_Blueprint_C"))
  (Variables|Default|SettargetActor _returnvalue))

(event Collision|EventActorBeginOverlap
  (params (OtherActor :type Actor%20Object%20Reference)))

(event EventTick
  (params (DeltaSeconds :type Float%20%28single-precision%29))
  (bind _targetactor (Variables|Default|GettargetActor))
  (Utilities|IsValid _targetactor
    (:Is%20Valid
      (AI|AIMoveTo self (Transformation|GetActorLocation _targetactor) 0 5e+01 false))))

(event Game|Damage|EventAnyDamage
  (params (Damage :type Float%20%28single-precision%29) (DamageType :type Damage%20Type%20Object%20Reference) (InstigatedBy :type Controller%20Object%20Reference) (DamageCauser :type Actor%20Object%20Reference))
  (Development|PrintString "Hello")
  (if (>= Damage (Variables|Default|GetcurrentHP))
    (Actor|DestroyActor)))

(fn ConstructionScript)